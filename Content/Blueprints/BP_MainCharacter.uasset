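; BP_MainCharacter is a player character that detects interactable actors in view and lets the player interact with them.
; A fast looping timer started on BeginPlay runs a sphere trace forward from the camera.
; Hits implementing BPI_Interaction are cached as TraceItem and notified when gaining or losing focus through CanReceiveTraceMessage.
; Pressing E sends InteractMessage to that item; BeginPlay also creates a UI_Interact widget without storing it.
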(event `Key|E`
  (params (Key :type "Key Structure"))
  (:`Pressed`
    (message `/Game/Blueprints/BPI_Interaction.Interact` (`self.Trace Item`))))

(event `Create Interaction Trace`
  (`self.Interaction Trace`))

(event `self.ReceiveBeginPlay`
  (`KismetSystemLibrary.K2_SetTimer` null)
  (bind _returnvalue (`KismetSystemLibrary.K2_SetTimer` null "Create Interaction Trace" 0.01 true))
  (set `self.Interaction Timer` _returnvalue)
  (`|CreateWidget` "/Game/Blueprints/UI_Interact.UI_Interact_C"))

(fn `Interaction Trace`
  (bind _cameracomponent (`self.CameraComponent`))
  (bind _returnvalue (`SceneComponent.K2_GetComponentLocation` _cameracomponent))
  (bind _outhit (`KismetSystemLibrary.SphereTraceSingle` _returnvalue (+ _returnvalue (* (`KismetMathLibrary.GetForwardVector` (`SceneComponent.K2_GetComponentRotation` _cameracomponent)) 1000.0)) 3.0 "TraceTypeQuery1"))
  (bind (_bblockinghit _binitialoverlap _time _distance _location _impactpoint _normal _impactnormal _physmat _hitactor) (`GameplayStatics.BreakHitResult` _outhit))
  (if (`KismetSystemLibrary.DoesImplementInterface` _hitactor "/Game/Blueprints/BPI_Interaction.BPI_Interaction_C")
    (if (!= _hitactor (`self.Trace Item`))
      (bind _output_get (set `self.Trace Item` _hitactor))
      (message `/Game/Blueprints/BPI_Interaction.Can Receive Trace` _output_get true))
    (else
      (message `/Game/Blueprints/BPI_Interaction.Can Receive Trace` (`self.Trace Item`) false)
      (set `self.Trace Item` null))))

(fn `UserConstructionScript`)